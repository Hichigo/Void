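; MainPlayerController is the player controller that owns and toggles the skill panel UI.
; BeginPlay creates the W_SkillPanel widget and adds it to the viewport.
; Q flip-flops the panel's WCanvasTree visibility, switching between Game and UI input focused on the panel and Game Only input.
; A debug Tab binding calls HealthIncrease on Stat.
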(event EventBeginPlay
  (Utilities|FlowControl|Sequence
    (:then_0
      (bind _returnvalue (UserInterface|CreateWidget "/Game/IslandOfTheVoid/UMG/SkillTree/W_SkillPanel.W_SkillPanel_C"))
      (bind _output_get (Variables|Default|SetSkillPanelRef _returnvalue))
      (UserInterface|Viewport|AddtoViewport _output_get 0))))

(event Input|KeyboardEvents|Tab
  (params (Key :type Key%20Structure :default "AnyKey"))
  ;[1 0 0] Debug
  (:Pressed
    (Class|StatComponent|HealthIncrease (Variables|Default|GetStat))))

(event Input|KeyboardEvents|Q
  (params (Key :type Key%20Structure :default "AnyKey"))
  (bind _skillpanelref (Variables|Default|GetSkillPanelRef))
  (bind _w_canvastree (Variables|/Game/IslandOfTheVoid/UMG/SkillTree/W_SkillPanel.W_SkillPanel_C|GetW_CanvasTree _skillpanelref))
  (:Pressed
    (Utilities|FlowControl|FlipFlop
      (:A
        (Widget|SetVisibility _w_canvastree "Visible")
        (Input|SetInputModeGameandUI self (Variables|Default|GetSkillPanelRef) "DoNotLock" false))
      (:B
        (Widget|SetVisibility _w_canvastree "Hidden")
        (Input|SetInputModeGameOnly self)))))

(fn ConstructionScript)