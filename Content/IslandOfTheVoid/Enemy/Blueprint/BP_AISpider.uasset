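; BP_AISpider is a spider enemy Blueprint that handles melee attacks against the player.
; PlayAnimationAttack turns it toward player 0, plays a random attack montage, then notifies the calling task after a delay from a separately randomized montage's length, which may differ.
; OnAttack line-traces forward within AttackRange for pawns, with debug drawing, and applies random damage from the MainStats range to the hit actor.
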(event Custom|OnAttack
  (bind _returnvalue (Transformation|GetActorLocation))
  (bind (_outhit _returnvalue_2) (Collision|LineTraceForObjects _returnvalue (+ _returnvalue (* (Transformation|GetActorForwardVector) (Variables|Default|GetAttackRange))) (Utilities|Array|MakeArray "ObjectTypeQuery3") false 0 "ForDuration"))
  (if _returnvalue_2
    (Game|Damage|ApplyDamage (.HitActor (Collision|BreakHitResult _outhit)) (CallFunction|GetDamage) 0 self)))

(event Custom|PlayAnimationAttack
  (params (TaskAttack :type BTT%20Attack%20Object%20Reference))
  (bind _animationsattack (Variables|Default|GetAnimationsAttack))
  (bind _returnvalue (Utilities|Array|Length _animationsattack))
  (bind _returnvalue_2 (Math|Random|RandomInteger _returnvalue))
  (bind _output (Utilities|Array|Get(acopy) _animationsattack _returnvalue_2))
  (Transformation|SetActorRotation (Math|Rotator|MakeRotator 0.0 0.0 (.Yaw (Math|Rotator|BreakRotator (Math|Rotator|FindLookatRotation (Transformation|GetActorLocation) (Transformation|GetActorLocation (Game|GetPlayerCharacter 0)))))))
  (Animation|PlayAnimMontage _output 1.0 "None")
  (Utilities|FlowControl|Delay (Variables|/Script/Engine.AnimSequenceBase|GetSequenceLength _output))
  (Default|EndAnimation TaskAttack))

(event EventBeginPlay)

(event Collision|EventActorBeginOverlap
  (params (OtherActor :type Actor%20Object%20Reference)))

(event EventTick
  (params (DeltaSeconds :type Float%20%28single-precision%29)))

(fn ConstructionScript)

(fn GetDamage
  (bind _mainstats (Variables|Default|GetMainStats))
  (bind _damage (Utilities|Struct|BreakEnemyStats _mainstats))
  (bind (_min _max) (Utilities|Struct|BreakDamage _damage))
  (return (Math|Random|RandomFloatinRange _min _max)))