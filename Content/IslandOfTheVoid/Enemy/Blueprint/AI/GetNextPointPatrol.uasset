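; Behavior tree task that feeds AI_Enemy pawns the next stop on their patrol route.
; It writes the location of the current PointsPatrol actor to the TargetLocation blackboard key, then advances its own NextPointIndex, looping to the first point after the last.
; It finishes successfully right away, but never calls FinishExecute if the pawn is not an AI_Enemy.
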(event EventReceiveExecuteAI
  (params (OwnerController :type AI%20Controller%20Object%20Reference) (ControlledPawn :type Pawn%20Object%20Reference))
  (bind _asai_enemy (Utilities|Casting|CastToAI_Enemy ControlledPawn))
  (AI|BehaviorTree|SetBlackboardValueasVector (Variables|Default|GetTargetLocation) (Transformation|GetActorLocation (Utilities|Array|Get(acopy) (Variables|/Game/IslandOfTheVoid/Enemy/Blueprint/AI_Enemy.AI_Enemy_C|GetPointsPatrol _asai_enemy) (Variables|Default|GetNextPointIndex))))
  (if (>= (Variables|Default|GetNextPointIndex) (Utilities|Array|LastIndex (Variables|/Game/IslandOfTheVoid/Enemy/Blueprint/AI_Enemy.AI_Enemy_C|GetPointsPatrol _asai_enemy)))
    (Variables|Default|SetNextPointIndex 0)
    (else
      (Math|Integer|IncrementInt (Variables|Default|GetNextPointIndex)
        (:%20%20
          _))))
  (AI|BehaviorTree|FinishExecute true))