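; AI controller for the spider enemy that switches it between chasing, searching and its default action based on perception of the player.
; Perception updates write the action state, player reference and last seen location to the Blackboard.
; Target updates also adjust walk speed per state.
; Losing the player starts a timer that, unless cancelled by a new sighting, restores the pawn's MainAction at a slower speed.
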(event OnTargetPerceptionUpdated(AIPerception)
  (params (Actor :type Actor%20Object%20Reference) (Stimulus :type AI%20Stimulus%20Structure))
  (if (== Actor (Game|GetPlayerCharacter 0))
    (if (.bsuccessfullysensed Stimulus)
      (Utilities|Time|ClearandInvalidateTimerbyHandle (Variables|Default|GetTimerLostPlayer))
      (Variables|/Script/Engine.CharacterMovementComponent|SetMaxWalkSpeed (Variables|/Script/Engine.Character|GetCharacterMovement (Variables|Default|GetSelfSpiderRef)) 5e+02)
      (AI|Components|Blackboard|SetValueasEnum (AI|GetBlackboard 0) (Variables|Default|GetBB_Action) (Variables|Default|GetChase))
      (else
        (AI|Components|Blackboard|SetValueasVector (AI|GetBlackboard 0) (Variables|Default|GetLastSeePlayerLocation) (Transformation|GetActorLocation Actor))
        (bind _returnvalue (Utilities|Time|SetTimerbyEvent (delegate Custom|ForgetPlayer) 15.0))
        (Variables|Default|SetTimerLostPlayer _returnvalue)
        (Variables|/Script/Engine.CharacterMovementComponent|SetMaxWalkSpeed (Variables|/Script/Engine.Character|GetCharacterMovement (Variables|Default|GetSelfSpiderRef)) 3.5e+02)
        (AI|Components|Blackboard|SetValueasEnum (AI|GetBlackboard 0) (Variables|Default|GetBB_Action) (Variables|Default|GetSearch))))))

(event OnPerceptionUpdated(AIPerception)
  (params (UpdatedActors :type Array%20of%20Actor%20Object%20References))
  (bind _returnvalue (AI|GetBlackboard 0))
  (bind _player (Variables|Default|GetPlayer))
  (for _array_element UpdatedActors
    (if (== _array_element (Game|GetPlayerCharacter 0))
      (bind _info (Class|AIPerceptionComponent|GetActorsPerception (Variables|Default|GetAIPerception) _array_element))
      (if (.bSuccessfullySensed (Utilities|Struct|BreakAIStimulus (Utilities|Array|Get(acopy) (.LastSensedStimuli (Utilities|Struct|BreakActorPerceptionBlueprintInfo _info)))))
        (AI|Components|Blackboard|SetValueasEnum (AI|GetBlackboard 0) (Variables|Default|GetBB_Action) (Variables|Default|GetChase))
        (AI|Components|Blackboard|SetValueasObject _returnvalue _player (.Target (Utilities|Struct|BreakActorPerceptionBlueprintInfo _info)))
        (else
          (AI|Components|Blackboard|SetValueasObject _returnvalue _player 0))))))

(event Custom|ForgetPlayer
  (AI|Components|Blackboard|SetValueasBool (AI|GetBlackboard 0) (Variables|Default|GetBB_Action) false)
  (Variables|/Script/Engine.CharacterMovementComponent|SetMaxWalkSpeed (Variables|/Script/Engine.Character|GetCharacterMovement (Variables|Default|GetSelfSpiderRef)) 2e+02)
  (AI|Components|Blackboard|SetValueasEnum (AI|GetBlackboard 0) (Variables|Default|GetBB_Action) (Variables|Default|GetMainAction)))

(event EventBeginPlay
  (bind _asai_enemy (Utilities|Casting|CastToAI_Enemy (Pawn|GetControlledPawn)))
  (bind _output_get (Variables|Default|SetSelfSpiderRef _asai_enemy))
  (Variables|Default|SetMainAction (Variables|/Game/IslandOfTheVoid/Enemy/Blueprint/AI_Enemy.AI_Enemy_C|GetMainAction _output_get)))

(fn ConstructionScript)